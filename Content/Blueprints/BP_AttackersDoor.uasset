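; BP_AttackersDoor is a door, named for the attackers, that slides its mesh open and closed.
; OpenDoor and CloseDoor use MoveComponentTo to shift MeshComp by plus or minus RelativeLocation over OpenTime or CloseTime, updating DoorState around each move.
; Both targets build on the mesh's current world location, though the move expects a relative location.
; An unconnected delayed chain calling CheckBeforeOpening and CheckBeforeClosing never runs.
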(event EventBeginPlay)

(event Collision|EventActorBeginOverlap
  (params (OtherActor :type Actor%20Object%20Reference)))

(event EventTick
  (params (DeltaSeconds :type Float%20%28single-precision%29)))

(event EventOpenDoor
  (Variables|Default|SetDoorState "Opening")
  (Components|MoveComponentTo (Variables|Default|GetMeshComp) (+ (Transformation|GetWorldLocation (Variables|Default|GetMeshComp)) (Variables|Default|GetRelativeLocation)) "0, 0, 0" false false (Variables|Default|GetOpenTime) false)
  (Variables|Default|SetDoorState "Opened"))

(event EventCloseDoor
  (Variables|Default|SetDoorState "Closing")
  (Components|MoveComponentTo (Variables|Default|GetMeshComp) (+ (* (Variables|Default|GetRelativeLocation) "-1.000000,-1.000000,-1.000000") (Transformation|GetWorldLocation (Variables|Default|GetMeshComp))) "0, 0, 0" false false (Variables|Default|GetCloseTime) false)
  (Variables|Default|SetDoorState "Closed"))

(fn ConstructionScript)