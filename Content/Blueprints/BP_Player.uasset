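; BP_Player is the player character Blueprint, which adds the game UI to the screen and carries movement tuning controls.
; BeginPlay creates WBP_GameUI for the local viewing player controller and adds it to the viewport if valid.
; The Add and Subtract keys step CharacterMovement's LedgeCheckThreshold up and down at runtime.
; Unconnected leftover nodes would print camera, crouch and threshold values or adjust PerchAdditionalHeight.
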(event EventBeginPlay
  (bind _returnvalue (UserInterface|CreateWidget "/Game/Blueprints/WBP_GameUI.WBP_GameUI_C" (Pawn|GetLocalViewingPlayerController)))
  (Utilities|IsValid _returnvalue
    (:Is%20Valid
      (UserInterface|Viewport|AddtoViewport _returnvalue 0))))

(event Collision|EventActorBeginOverlap
  (params (OtherActor :type Actor%20Object%20Reference)))

(event EventTick
  (params (DeltaSeconds :type Float%20%28single-precision%29)))

(event Input|KeyboardEvents|Escape
  (params (Key :type Key%20Structure :default "None")))

(event Input|KeyboardEvents|Add
  (params (Key :type Key%20Structure :default "None"))
  (bind _charactermovement (Variables|Character|GetCharacterMovement))
  (:Pressed
    (Variables|/Script/Engine.CharacterMovementComponent|SetLedgeCheckThreshold _charactermovement (+ (Variables|/Script/Engine.CharacterMovementComponent|GetLedgeCheckThreshold _charactermovement) 1.0))))

(event Input|KeyboardEvents|NumPadNine
  (params (Key :type Key%20Structure :default "None")))

(event Input|KeyboardEvents|Subtract
  (params (Key :type Key%20Structure :default "None"))
  (bind _charactermovement (Variables|Character|GetCharacterMovement))
  (:Pressed
    (Variables|/Script/Engine.CharacterMovementComponent|SetLedgeCheckThreshold _charactermovement (+ (Variables|/Script/Engine.CharacterMovementComponent|GetLedgeCheckThreshold _charactermovement) -1.0))))

(event Input|KeyboardEvents|NumPadSix
  (params (Key :type Key%20Structure :default "None")))

(fn ConstructionScript)